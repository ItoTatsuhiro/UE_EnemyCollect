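; BP_ExampleSword is a display actor that shows an elemental sword as an animated, floating crystal with a particle effect.
; The construction script and BeginPlay both apply the configurable sword mesh and particle template.
; Tick spins PortalCrystal about Z, swivels MainCrystal using rotated axis vectors and bobs it vertically on a sine wave.
; Helpers MakeSine and MakeBobbing hold the same cycle and sine math that appears inline in Tick.
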(event EventBeginPlay
  ;[1 1 1] Begin Play
  (Components|StaticMesh|SetStaticMesh (Variables|Default|GetMainCrystal) (Variables|Default|GetSword%20Mesh))
  (Effects|Components|ParticleSystem|SetTemplate (Variables|Default|GetParticleSystem) (Variables|Default|GetParticle)))

(event EventTick
  (params (DeltaSeconds :type Float%20%28single-precision%29))
  (bind _returnvalue (* DeltaSeconds 3.6e+02))
  (bind _maincrystal (Variables|Default|GetMainCrystal))
  ;[1 1 1] AnimSet
  (|CallParentFunction DeltaSeconds)
  (Transformation|AddRelativeRotation (Variables|Default|GetPortalCrystal) (Math|Vector|RotatorfromAxisandAngle "0,0.000000,1.000000" (* DeltaSeconds (Variables|Default|GetRotationSpeed))) false false)
  ;;[0 0 0] Progress swivel angle
  (Variables|Swivel|SetCurrent%20Swivel%20X (Math|Float|%(Float) (+ (/ _returnvalue (Variables|Swivel|GetSwivel%20Cone%20X)) (Variables|Swivel|GetCurrent%20Swivel%20X)) 3.6e+02))
  (Variables|Swivel|SetCurrent%20Swivel%20Y (Math|Float|%(Float) (+ (/ _returnvalue (Variables|Swivel|GetSwivel%20Cone%20Y)) (Variables|Swivel|GetCurrent%20Swivel%20Y)) 3.6e+02))
  (Transformation|SetRelativeRotation _maincrystal (Math|Rotator|MakeRotfromXY (Math|Vector|RotateVectorAroundAxis (Variables|Swivel|GetSwivel%20Axis%20X) (Variables|Swivel|GetCurrent%20Swivel%20X) "1.000000, 0, 0") (Math|Vector|RotateVectorAroundAxis (Variables|Swivel|GetSwivel%20Axis%20Y) (Variables|Swivel|GetCurrent%20Swivel%20Y) "0,1.000000, 0")) false false)
  (Utilities|FlowControl|Sequence
    (:then_0
      ;;[0 0 0] Progress bobbing cycles
      (Variables|Bobbing|SetBobbing%20Cycle%201 (Math|Float|%(Float) (+ (Variables|Bobbing|GetBobbing%20Cycle%201) (/ (* (Utilities|Time|GetWorldDeltaSeconds) 3.6e+02) (Variables|Bobbing|GetBobbing%20Period%201))) 3.6e+02)))
    (:then_1
      (Transformation|SetRelativeLocation _maincrystal (+ (Variables|CrystalLocation|GetMainCrystal_Location) (Math|Vector|MakeVector 0.0 0.0 (* (Variables|Bobbing|GetBobbing%20Amplitude%201) (Math|Trig|Sin(Degrees) (Variables|Bobbing|GetBobbing%20Cycle%201))))) false false))))

(fn ConstructionScript
  (Components|StaticMesh|SetStaticMesh (Variables|Default|GetMainCrystal) (Variables|Default|GetSword%20Mesh))
  (Effects|Components|ParticleSystem|SetTemplate (Variables|Default|GetParticleSystem) (Variables|Default|GetParticle)))

(fn MakeSine
  (params (Period :type Float%20%28double-precision%29) (Cycle :type Float%20%28double-precision%29))
  (return (Math|Float|%(Float) (+ Cycle (/ (* (Utilities|Time|GetWorldDeltaSeconds) 3.6e+02) Period)) 3.6e+02)))

(fn MakeBobbing
  (params (Amplitude :type Float%20%28double-precision%29) (Cycle :type Float%20%28double-precision%29))
  (return (* Amplitude (Math|Trig|Sin(Degrees) Cycle))))