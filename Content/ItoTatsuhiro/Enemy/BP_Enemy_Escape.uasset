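; Enemy character Blueprint that carries a child-actor weapon, takes damage and drops a BP_Item when killed.
; On BeginPlay it adds ATK to the weapon's damage, initializes the HP text widget and raises PlaySceneManager's item maximum by one.
; AnyDamage updates HP, then plays a hit montage or triggers death, which ragdolls the mesh, stops AI logic, waits, spawns the item and destroys the actor.
; Attack only plays a melee montage.
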(event Custom|Attack
  ;[1 1 1] 攻撃
  (Animation|Montage|PlayMontage (Variables|Character|GetMesh) "/Game/ItoTatsuhiro/Anim/Standing_Melee_Attack_Downward__1__Anim_mixamo_com1_Montage.Standing_Melee_Attack_Downward__1__Anim_mixamo_com1_Montage"))

(event Custom|Death
  ;[1 1 1] 死亡時の処理
  (Class|SkeletalMeshComponent|SetAllBodiesSimulatePhysics (Variables|Character|GetMesh) true)
  (Collision|SetCollisionEnabled (Variables|Character|GetMesh) "PhysicsOnly")
  (AI|Logic|StopLogic (Variables|/Script/AIModule.AIController|GetBrainComponent (AI|GetAIController self)) "")
  (Utilities|FlowControl|Delay 3.0)
  (Game|SpawnActorfromClass "/Game/MaeTakuto/Object/BP_Item.BP_Item_C" (Transformation|GetActorTransform) "Undefined" 0 0)
  (Actor|DestroyActor))

(event Game|Damage|EventAnyDamage
  (params (Damage :type Float%20%28single-precision%29) (DamageType :type Damage%20Type%20Object%20Reference) (InstigatedBy :type Controller%20Object%20Reference) (DamageCauser :type Actor%20Object%20Reference))
  ;[1 1 1] ダメージ処理
  (bind _output_get (Variables|Default|SetHP (- (Variables|Default|GetHP) Damage)))
  ;;[1 1 1] HPバーのセット
  (bind _asenemy_hpbar (Utilities|Casting|CastToenemy_HPbar (UserInterface|GetUserWidgetObject (Variables|Default|GetHP_Bar))))
  (Rendering|Components|TextRender|SetText (Variables|/Game/wadatomoya/UI/enemy_HPbar.enemy_HPbar_C|GetTextBlock_73 _asenemy_hpbar) (Utilities|Text|ToText(Float) (Math|Float|Max(Float) (Variables|Default|GetHP) 0.0) "HalfToEven"))
  (if (<= _output_get 0.0)
    (Development|PrintString "やられた")
    (CallFunction|Death)
    (else
      (Development|PrintString "ダメージが入った")
      (Animation|Montage|PlayMontage (Variables|Character|GetMesh) "/Game/ItoTatsuhiro/Anim/damage/Damage_Montage.Damage_Montage"))))

(event EventBeginPlay
  ;[1 1 1] ゲーム開始時
  ;;[1 1 1] 自身の攻撃力をBaseWeaponに反映
  (bind _asbase_weapon (Utilities|Casting|CastToBaseWeapon (Variables|/Script/Engine.ChildActorComponent|GetChildActor (Variables|Default|GetChildActor))))
  (bind _output_get (Variables|/Game/ItoTatsuhiro/BP/BaseWeapon.BaseWeapon_C|Setdamage _asbase_weapon (+ (Variables|Default|GetATK) (Variables|/Game/ItoTatsuhiro/BP/BaseWeapon.BaseWeapon_C|Getdamage _asbase_weapon))))
  (Development|PrintString (Utilities|String|ToString(Float) _output_get))
  ;;[1 1 1] HPバーの初期化
  (bind _asenemy_hpbar (Utilities|Casting|CastToenemy_HPbar (UserInterface|GetUserWidgetObject (Variables|Default|GetHP_Bar))))
  (Rendering|Components|TextRender|SetText (Variables|/Game/wadatomoya/UI/enemy_HPbar.enemy_HPbar_C|GetTextBlock_73 _asenemy_hpbar) (Utilities|Text|ToText(Float) (Variables|Default|GetHP) "HalfToEven"))
  (Actor|SetOwner (Variables|/Script/Engine.ChildActorComponent|GetChildActor (Variables|Default|GetChildActor)) self)
  (bind _returnvalue (Actor|GetActorOfClass "/Game/ItoTatsuhiro/BP/UI/PlaySceneManager.PlaySceneManager_C"))
  (Default|AddItemMax _returnvalue 1))

(fn ConstructionScript)