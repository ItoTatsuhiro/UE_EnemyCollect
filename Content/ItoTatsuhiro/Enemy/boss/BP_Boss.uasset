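; BP_Boss is a boss enemy that takes damage and fires bullets at the player character.
; On BeginPlay it copies default HP, ATK and SPD into working values and caches the BP_ThirdPersonCharacter as Player.
; AnyDamage subtracts from HP and only prints a hit or defeat message.
; The Attack event spawns BP_BossBullet at the Canon transform, passing it the player's current location and the boss capsule's rotation.
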(event Custom|Attack
  ;[1 1 1] 攻撃(弾の発射)
  (bind _returnvalue (Game|SpawnActorfromClass "/Game/ItoTatsuhiro/Enemy/boss/BP_BossBullet.BP_BossBullet_C" (Transformation|GetWorldTransform (Variables|Default|GetCanon)) "Undefined" 0 0))
  (Default|SetValue _returnvalue (Transformation|GetActorLocation (Variables|Default|Getplayer)) (Variables|/Script/Engine.SceneComponent|GetRelativeRotation (Variables|Collision|GetCapsuleComponent))))

(event Game|Damage|EventAnyDamage
  (params (Damage :type Float%20%28single-precision%29) (DamageType :type Damage%20Type%20Object%20Reference) (InstigatedBy :type Controller%20Object%20Reference) (DamageCauser :type Actor%20Object%20Reference))
  ;[1 1 1] ダメージ処理
  (bind _output_get (Variables|Default|SetHP (- (Variables|Default|GetHP) Damage)))
  (if (<= _output_get 0.0)
    (Development|PrintString "ボスがやられた")
    (else
      (Development|PrintString "ボスにダメージが入った"))))

(event EventBeginPlay
  (Variables|Default|SetHP (Variables|Default|GetHP_Default))
  (Variables|Default|SetATK (Variables|Default|GetATK_Default))
  (Variables|Default|SetSPD (Variables|Default|GetSPD_Default))
  (bind _returnvalue (Actor|GetActorOfClass "/Game/ThirdPerson/Blueprints/BP_ThirdPersonCharacter.BP_ThirdPersonCharacter_C"))
  (Variables|Default|Setplayer _returnvalue))

(fn ConstructionScript)