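; BP_BossBullet is a boss projectile that flies toward a target position and damages actors outside its group.
; SetValue stores target, spawner rotation and group tag, then sets ProjectileMovement velocity.
; The direction is counter-rotated by the spawner's rotation because velocity is set in local space.
; Sphere overlaps compare group tags and apply damage through a delay-reset DoOnce, without destroying the bullet.
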(event OnComponentBeginOverlap(Sphere)
  (params (OverlappedComponent :type Primitive%20Component%20Object%20Reference) (OtherActor :type Actor%20Object%20Reference) (OtherComp :type Primitive%20Component%20Object%20Reference) (OtherBodyIndex :type Integer) (bFromSweep :type Boolean) (SweepResult :type Hit%20Result%20Structure%20%28by%20ref%29))
  (bind _damage (Variables|Default|Getdamage))
  (bind _grouptag (Class|BPIGetGroupTag|GetGroupTag(Message) OtherActor))
  (if (Utilities|Enum|NotEqual(Enum) _grouptag (Variables|Default|GetGroup%20Tag))
    (Utilities|FlowControl|DoOnce false :!label _label
      (:Completed
        (Game|Damage|ApplyDamage OtherActor _damage 0 0)
        (Development|PrintString (Utilities|String|ToString(Float) _damage))
        (Utilities|FlowControl|Delay 0.5)
        (goto _label Reset)))))

(event Custom|SetVelocity
  (bind _projectilemovement (Variables|Default|GetProjectileMovement))
  ;[1 1 1] 弾の進む方向を計算する
  (Game|Components|ProjectileMovement|SetVelocityinLocalSpace _projectilemovement (* (Math|Vector|Normalize (Math|Vector|RotateVector (- (Variables|Default|GettargetPos) (Transformation|GetWorldLocation (Variables|Default|GetStaticMesh))) (Class|KismetMathLibrary|NegateRotator (Variables|Default|GetmakerRotation)))) (Variables|/Script/Engine.ProjectileMovementComponent|GetInitialSpeed _projectilemovement))))

(fn ConstructionScript)

(fn SetValue
  (params (target :type Vector) (makerRotation :type Rotator) (groupTag :type Enum_GroupTag%20Enum :default "NewEnumerator0"))
  (Variables|Default|SettargetPos target)
  (Variables|Default|SetmakerRotation makerRotation)
  (Variables|Default|SetGroup%20Tag groupTag)
  (CallFunction|SetVelocity))

(fn GetGroupTag
  (return (Variables|Default|GetGroup%20Tag)))