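; BP_Bullet is a boss enemy projectile that aims at the player once, on spawn.
; BeginPlay passes the normalized mesh-to-player direction, unscaled, to ProjectileMovement as a local-space velocity, although it is computed in world space.
; On hit, it pushes physics-simulating components with an impulse scaled from its velocity, then destroys itself.
; Other hits are ignored, and no damage is applied.
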(event Custom|setVector
  (Game|Components|ProjectileMovement|SetVelocityinLocalSpace (Variables|Default|GetProjectileMovement) (Math|Vector|Normalize (- (Transformation|GetWorldLocation (Variables|/Script/Engine.Character|GetMesh (Game|GetPlayerCharacter 0))) (Transformation|GetWorldLocation (Variables|Default|GetStaticMesh))))))

(event EventBeginPlay
  (CallFunction|SetVector))

(event Collision|EventHit
  (params (MyComp :type Primitive%20Component%20Object%20Reference) (Other :type Actor%20Object%20Reference) (OtherComp :type Primitive%20Component%20Object%20Reference) (bSelfMoved :type Boolean) (HitLocation :type Vector :default "0, 0, 0") (HitNormal :type Vector :default "0, 0, 0") (NormalImpulse :type Vector :default "0, 0, 0") (Hit :type Hit%20Result%20Structure%20%28by%20ref%29))
  (if (Physics|IsSimulatingPhysics OtherComp "None")
    (Physics|AddImpulseatLocation OtherComp (* (Transformation|GetVelocity) "100.000000,100.000000,100.000000") (Transformation|GetActorLocation) "None")
    (Actor|DestroyActor)))

(fn ConstructionScript)