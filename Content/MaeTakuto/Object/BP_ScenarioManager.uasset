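; BP_ScenarioManager tracks the current scenario chapter and supplies that chapter's scenario data table.
; On BeginPlay it counts the rows of ChapterDataTable to find the last page, then sets NowChapter from BP_GameInstance_wada's saved chapter value.
; SetNowChapter rejects values above the last page with a warning.
; GetNowChapterScenario looks up the row named after the chapter number and returns its ChapterScenarioData.
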(event EventBeginPlay
  (CallFunction|CheckLastPage) ; 最終チャプターを確認し、設定する。
  ;[1 1 1] 現在のシナリオチャプターを取得して、設定する
  (bind _asbp_game_instance_wada (Utilities|Casting|CastToBP_GameInstance_wada (Game|GetGameInstance))
    (:then
      (Development|PrintString (Utilities|String|Append "現在のチャプター：" (Utilities|String|ToString(Integer) (Variables|/Game/wadatomoya/gameinstance/BP_GameInstance_wada.BP_GameInstance_wada_C|GetNow%20Scenario%20Chapter _asbp_game_instance_wada))))
      (CallFunction|SetNowChapter (Variables|/Game/wadatomoya/gameinstance/BP_GameInstance_wada.BP_GameInstance_wada_C|GetNow%20Scenario%20Chapter _asbp_game_instance_wada)))
    (:CastFailed
      (Development|PrintString "ScenatioManager：GameInstanceを取得できませんでした。" true true "(R=1.000000,G=0.000000,B=0.000000,A=1.000000)") ; エラーを出力
    )))

(event Collision|EventActorBeginOverlap
  (params (OtherActor :type Actor%20Object%20Reference)))

(event EventTick
  (params (DeltaSeconds :type Float%20%28single-precision%29)))

(fn ConstructionScript)

(fn GetNowChapterScenario
  (bind _nowchapter (Variables|Default|GetNowChapter))
  (bind _returnvalue (Utilities|String|ToString(Integer) _nowchapter))
  (Development|PrintString (Utilities|String|Append "取得したチャプター：" _returnvalue))
  (bind _returnvalue_2 (Utilities|GetDataTableRow (Variables|Default|GetChapterDataTable) (Utilities|String|StringToName _returnvalue))
    (:then
      (bind _output_get (LocalVariables|SetDataTable (.ChapterScenarioData (Utilities|Struct|BreakAllChapterDataStruct _returnvalue_2))))
      (Development|PrintString (Utilities|String|Append "取得したチャプター：" (Utilities|String|ToString(Integer) (.Chapter (Utilities|Struct|BreakAllChapterDataStruct _returnvalue_2)))))
      (return _output_get))))

(fn SetNowChapter
  (params (Chapter :type Integer))
  (if (> Chapter (Variables|Default|GetLastPage)) ; NextChapterが最終行か判定する
    (Development|PrintString (Utilities|String|Append "ScenaripManager：Chapterの切り替えができませんでした。入力値：" (Utilities|String|ToString(Integer) Chapter)) true true "(R=1.000000,G=1.000000,B=0.000000,A=1.000000)")
    (else
      (bind _output_get (Variables|Default|SetNowChapter Chapter))
      (Development|PrintString (Utilities|String|Append "NowChapterを変更しました。　変更値：" (Utilities|String|ToString(Integer) _output_get))))))

(fn CheckLastPage
  (bind _outrownames (DataTable|GetDataTableRowNames (Variables|Default|GetChapterDataTable)))
  (for _array_element _outrownames
    (Math|Integer|IncrementInt (Variables|Default|GetLastPage))))