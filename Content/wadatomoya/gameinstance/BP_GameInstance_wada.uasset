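; Game instance that holds the Quest 1 clear flag and persists it through BP_SaveGame.
; On Init it creates a save object in memory only if the slot is empty, so an existing save is referenced only after LoadGameData runs.
; Quest1Clear sets the flag and SaveGameData writes it to the slot.
; LoadGameData returns the saved value without copying it back into IsQuest1clear.
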(event EventInit
  ;[1 1 1] ゲーム起動時SaveGameがなければSaveGameを作る
  (bind _returnvalue (SaveGame|DoesSaveGameExist (Variables|Default|GetSlot%20Name)))
  (if (not _returnvalue)
    (bind _returnvalue_2 (SaveGame|CreateSaveGameObject "/Game/wadatomoya/savegame/BP_SaveGame.BP_SaveGame_C"))
    (Variables|Default|SetSaveGameRef _returnvalue_2)))

(fn Quest1Clear
  (Variables|Default|SetisQuest1clear%20 true))

(fn SaveGameData
  (bind _savegameref (Variables|Default|GetSaveGameRef))
  (Variables|/Game/wadatomoya/savegame/BP_SaveGame.BP_SaveGame_C|SetClearQuest1 _savegameref (Variables|Default|GetisQuest1clear%20))
  (SaveGame|SaveGametoSlot _savegameref (Variables|Default|GetSlot%20Name)))

(fn LoadGameData
  (bind _returnvalue (SaveGame|LoadGamefromSlot (Variables|Default|GetSlot%20Name)))
  (bind _asbp_save_game (Utilities|Casting|CastToBP_SaveGame _returnvalue))
  (bind _output_get (Variables|Default|SetSaveGameRef _asbp_save_game))
  (return (Variables|/Game/wadatomoya/savegame/BP_SaveGame.BP_SaveGame_C|GetClearQuest1 _output_get)))