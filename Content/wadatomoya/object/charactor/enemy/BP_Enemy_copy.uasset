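; Enemy character Blueprint that tracks HP, reacts to damage and plays a melee attack animation.
; BeginPlay and AnyDamage write the HP value as text into the enemy_HPbar of its widget component.
; AnyDamage subtracts from HP, then plays a hit montage, or only prints a defeat message once HP drops below zero.
; The Attack event just plays a downward melee montage, with no damage logic.
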(event Custom|Attack
  ;[1 1 1] 攻撃
  (Animation|Montage|PlayMontage (Variables|Character|GetMesh) "/Game/ItoTatsuhiro/Anim/Standing_Melee_Attack_Downward__1__Anim_mixamo_com1_Montage.Standing_Melee_Attack_Downward__1__Anim_mixamo_com1_Montage"))

(event Game|Damage|EventAnyDamage
  (params (Damage :type Float%20%28single-precision%29) (DamageType :type Damage%20Type%20Object%20Reference) (InstigatedBy :type Controller%20Object%20Reference) (DamageCauser :type Actor%20Object%20Reference))
  ;[1 1 1] ダメージ処理
  (bind _output_get (Variables|Default|SetHP (- (Variables|Default|GetHP) Damage)))
  (bind _asenemy_hpbar (Utilities|Casting|CastToenemy_HPbar (UserInterface|GetUserWidgetObject (Variables|Default|GetWidget))))
  (Rendering|Components|TextRender|SetText (Variables|/Game/wadatomoya/UI/enemy_HPbar.enemy_HPbar_C|GetTextBlock_73 _asenemy_hpbar) (Utilities|Text|ToText(Float) (Variables|Default|GetHP) "HalfToEven"))
  (if (< _output_get 0.0)
    (Development|PrintString "やられた")
    (else
      (Development|PrintString "ダメージが入った")
      (Animation|Montage|PlayMontage (Variables|Character|GetMesh) "/Game/ItoTatsuhiro/Anim/damage/Damage_Montage.Damage_Montage"))))

(event EventBeginPlay
  (bind _asenemy_hpbar (Utilities|Casting|CastToenemy_HPbar (UserInterface|GetUserWidgetObject (Variables|Default|GetWidget))))
  (Rendering|Components|TextRender|SetText (Variables|/Game/wadatomoya/UI/enemy_HPbar.enemy_HPbar_C|GetTextBlock_73 _asenemy_hpbar) (Utilities|Text|ToText(Float) (Variables|Default|GetHP) "HalfToEven")))

(fn ConstructionScript)